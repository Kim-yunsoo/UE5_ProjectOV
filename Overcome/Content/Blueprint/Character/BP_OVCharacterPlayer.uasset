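; Player character Blueprint whose only working logic is a shield-sphere toggle and a debug print key.
; Tick hides the Sphere and disables its collision while IsActiveShieldSkill is true, and restores both otherwise.
; A self-looping CameraSpin event yaws the control rotation, but its only call is disconnected.
; Grenade throwing with a predicted spline-mesh trajectory, plus shake, damage, noise and outline snippets, remain as unwired nodes that never run.
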(event Custom|CameraSpin
  (bind _returnvalue (Game|GetPlayerController 0))
  (bind _returnvalue_2 (Pawn|GetControlRotation _returnvalue :!class /Script/Engine.Controller))
  (Pawn|SetControlRotation (Game|GetPlayerController 0) (Math|Rotator|MakeRotator (.roll _returnvalue_2) (.pitch _returnvalue_2) (+ (.yaw _returnvalue_2) 0.2)))
  (Utilities|FlowControl|Delay 0.001)
  (CallFunction|CameraSpin))

(event Custom|ShowProjectilePath
  ;[1 1 1] Path
)

(event Input|EnhancedActionEvents|EnhancedInputActionIA_OV_Grenade
  (params (ActionValue :type Boolean) (ElapsedSeconds :type Float%20%28double-precision%29) (TriggeredSeconds :type Float%20%28double-precision%29) (InputAction :type Input%20Action%20Object%20Reference :default "/Game/Input/Actions/IA_OV_Grenade.IA_OV_Grenade"))
  ;[1 1 1] Grenade
)

(event EventBeginPlay)

(event Collision|EventActorBeginOverlap
  (params (OtherActor :type Actor%20Object%20Reference)))

(event EventTick
  (params (DeltaSeconds :type Float%20%28single-precision%29))
  (if (Variables|Default|GetbIsActiveShieldSkill)
    (Rendering|SetVisibility (Variables|Default|GetSphere) false false)
    (Collision|SetCollisionEnabled (Variables|Default|GetSphere) "NoCollision")
    (Collision|SetCollisionObjectType (Variables|Default|GetSphere) "ECC_Pawn")
    (else
      (Rendering|SetVisibility (Variables|Default|GetSphere) true false)
      (Collision|SetCollisionEnabled (Variables|Default|GetSphere) "QueryAndPhysics")
      (Collision|SetCollisionObjectType (Variables|Default|GetSphere) "ECC_Pawn"))))

(event Input|KeyboardEvents|X
  (params (Key :type Key%20Structure :default "None")))

(event Input|KeyboardEvents|G
  (params (Key :type Key%20Structure :default "None")))

(event Input|KeyboardEvents|1
  (params (Key :type Key%20Structure :default "None"))
  (:Pressed
    (Development|PrintString "Hello")))

(fn ConstructionScript)