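; BP_Cube is a cube actor that reacts once to an explosion hit, then removes itself.
; OnExplosionHit passes through a DoOnce, prints the actor name and damage, hides the static mesh and switches its collision to physics only.
; A short lifespan then destroys the actor, and the damage value is only printed, with no health tracking.
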(event EventBeginPlay)

(event Collision|EventActorBeginOverlap
  (params (OtherActor :type Actor%20Object%20Reference)))

(event EventTick
  (params (DeltaSeconds :type Float%20%28single-precision%29)))

(event EventOnExplosionHit
  (params (Explosion%20Source :type Actor%20Object%20Reference) (Damage :type Float%20%28double-precision%29))
  (Utilities|FlowControl|DoOnce false
    (:Completed
      (Development|PrintString (Utilities|String|Append (Utilities|GetDisplayName self) ":    event" (Utilities|String|ToString(Float) Damage)))
      (Development|SetHiddeninGame (Variables|Debug|GetStaticMeshComponent) true false)
      (Collision|SetCollisionEnabled (Variables|Debug|GetStaticMeshComponent) "PhysicsOnly")
      (Actor|SetLifeSpan 5.0))))

(fn ConstructionScript)