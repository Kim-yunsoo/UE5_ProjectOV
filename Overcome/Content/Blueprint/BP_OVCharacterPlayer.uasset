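; Player character Blueprint for third-person item pickup, aiming and shooting.
; F sends a pickup message to overlapping BP_Item actors and reveals the child-actor gun.
; Right mouse shows the target UI, follows controller yaw, clamps pitch and eases the camera between CameraBoom and SpringArm.
; Left mouse starts fire when IsAiming, which is never set here, passing a camera line-trace impact point, and stops on release.
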(event EventBeginPlay
  (bind _returnvalue (UserInterface|CreateWidget "/Game/UMG/TargetUI.TargetUI_C" 0 self))
  (bind _output_get (Variables|Default|SetUI _returnvalue))
  (UserInterface|Viewport|AddtoViewport _output_get 0)
  (Widget|SetVisibility (Variables|Default|GetUI) "Hidden"))

(event Collision|EventActorBeginOverlap
  (params (OtherActor :type Actor%20Object%20Reference)))

(event EventTick
  (params (DeltaSeconds :type Float%20%28single-precision%29)))

(event Input|MouseEvents|RightMouseButton
  (params (Key :type Key%20Structure :default "None"))
  (bind _returnvalue (Game|GetPlayerCameraManager 0))
  (:Pressed
    (Widget|SetVisibility (Variables|Default|GetUI) "Visible")
    (Variables|Default|SetbUseControllerRotationYaw true)
    (Variables|/Script/Engine.PlayerCameraManager|SetViewPitchMin _returnvalue -5e+01)
    (Variables|/Script/Engine.PlayerCameraManager|SetViewPitchMax _returnvalue 5e+01)
    (Transformation|AttachComponentToComponent (Variables|Default|GetFollowCamera) (Variables|Default|GetSpringArm) "None" "KeepWorld" "KeepWorld" "KeepWorld" true)
    (Components|MoveComponentTo (Variables|Default|GetFollowCamera) "0, 0, 0" "0, 0, 0" true true 0.5 true :!label _label))
  (:Released
    (Widget|SetVisibility (Variables|Default|GetUI) "Hidden")
    (Variables|Default|SetbUseControllerRotationYaw false)
    (Transformation|AttachComponentToComponent (Variables|Default|GetFollowCamera) (Variables|Default|GetCameraBoom) "None" "KeepWorld" "KeepWorld" "KeepWorld" true)
    (goto _label)))

(event Input|KeyboardEvents|F
  (params (Key :type Key%20Structure :default "None"))
  (:Pressed
    (for _array_element (Collision|GetOverlappingActors "/Game/PickUpSystem/BP_Item.BP_Item_C" :!class /Script/Engine.Actor)
      (if (Utilities|DoesObjectImplementInterface _array_element "/Game/PickUpSystem/BPI_Items.BPI_Items_C")
        (Class|BPIItems|PickUp(Message) _array_element)
        (Rendering|SetVisibility (Variables|Default|GetBP_Gun) true false)))))

(event Input|MouseEvents|LeftMouseButton
  (params (Key :type Key%20Structure :default "None"))
  (:Pressed
    (if (Variables|Default|GetbIsAiming)
      (Class|BPIFire|Fire(Message) (Variables|/Script/Engine.ChildActorComponent|GetChildActor (Variables|Default|GetBP_Gun)) true (CallFunction|GetTargetLocation))))
  (:Released
    (Class|BPIFire|Fire(Message) (Variables|/Script/Engine.ChildActorComponent|GetChildActor (Variables|Default|GetBP_Gun)) false "0, 0, 0")))

(fn ConstructionScript)

(fn GetTargetLocation
  (bind _followcamera (Variables|Default|GetFollowCamera))
  (bind _returnvalue (Transformation|GetSocketLocation _followcamera "None"))
  (bind _outhit (Collision|LineTraceByChannel _returnvalue (+ _returnvalue (* (Math|Vector|GetForwardVector (Pawn|GetControlRotation (Game|GetPlayerController 0) :!class /Script/Engine.Controller)) 1e+09)) "TraceTypeQuery1" false 0 "None"))
  (return (.ImpactPoint (Collision|BreakHitResult _outhit))))